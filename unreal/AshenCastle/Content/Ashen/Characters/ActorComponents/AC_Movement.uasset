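; AC_Movement is an actor component that moves its owning Character from a two-axis movement input.
; On BeginPlay it casts and caches the owner as a Character, printing an error if the cast fails.
; ApplyMovementInput feeds X along the right vector and Y along the forward vector of the control yaw, as forced movement input.
; Debug prints report the owner's name and each input received.
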(event EventBeginPlay
  (bind _returnvalue (Components|GetOwner))
  (bind _ascharacter (Utilities|Casting|CastToCharacter _returnvalue)
    (:then
      (bind _output_get (Variables|Default|SetownerCharacter _ascharacter))
      (Development|PrintString (Utilities|GetDisplayName _output_get)))
    (:CastFailed
      (Development|PrintText (Utilities|Text|FormatText "Failed to cast target to character: {owner}" _returnvalue)))))

(event EventApplyMovementInput
  (params (Input :type Vector%202D%20Structure))
  (bind (_x _y) (Math|Vector2D|BreakVector2D Input))
  (bind _ownercharacter (Variables|Default|GetownerCharacter))
  (bind _ownercharacter_2 (Variables|Default|GetownerCharacter))
  (bind _returnvalue (Pawn|GetControlRotation _ownercharacter :!class /Script/Engine.Pawn))
  (bind _yaw (Math|Rotator|BreakRotator _returnvalue))
  (bind _returnvalue_2 (Math|Rotator|MakeRotator 0.0 0.0 _yaw))
  (Development|PrintString (Utilities|String|ToString(Vector2d) Input))
  (Development|PrintString (Utilities|GetDisplayName _ownercharacter_2))
  (Pawn|Input|AddMovementInput _ownercharacter_2 (Math|Vector|GetRightVector _returnvalue_2) _x true)
  (Pawn|Input|AddMovementInput _ownercharacter_2 (Math|Vector|GetForwardVector _returnvalue_2) _y true))