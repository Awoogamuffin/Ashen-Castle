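; Base actor component that turns its owning character to face a target, leaving HandleLook empty as a likely hook for child components.
; LookAtTarget builds a yaw-only rotation toward a world position and passes it to RotateTowards.
; RotateTowards accelerates TurnSpeed toward its maximum for constant-rate turning.
; Within a yaw threshold that scales with TurnSpeed, it decelerates TurnSpeed toward zero and switches to eased interpolation.
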(event EventBeginPlay
  (|CallParentFunction))

(event EventTick
  (params (DeltaSeconds :type Float%20%28single-precision%29)))

(fn LookatTarget
  (params (TargetPosition :type Vector))
  (CallFunction|RotateTowards (Math|Rotator|MakeRotator 0.0 0.0 (.Yaw (Math|Rotator|BreakRotator (Math|Rotator|FindLookatRotation (Transformation|GetActorLocation (Variables|Default|GetOwnerCharacter)) TargetPosition))))))

(fn HandleLook)

(fn RotateTowards
  (params (target :type Rotator))
  (bind _ownercharacter (Variables|Default|GetOwnerCharacter))
  (if (< (Math|Float|Absolute(Float) (.Yaw (Math|Rotator|BreakRotator (Math|Rotator|Delta(Rotator) (Transformation|GetActorRotation (Variables|Default|GetOwnerCharacter)) target)))) (/ (Variables|Default|GetTurnSpeed) 1e+01))
    (Variables|Default|SetTurnSpeed (Math|Interpolation|FInterptoConstant (Variables|Default|GetTurnSpeed) 0.0 (Utilities|Time|GetWorldDeltaSeconds) (Variables|Default|GetTurnSpeedAcc)))
    (Transformation|SetActorRotation _ownercharacter (Math|Interpolation|RInterpTo (Transformation|GetActorRotation _ownercharacter) target (Utilities|Time|GetWorldDeltaSeconds) 5.0))
    (else
      (Variables|Default|SetTurnSpeed (Math|Interpolation|FInterptoConstant (Variables|Default|GetTurnSpeed) (Variables|Default|GetTurnSpeedMax) (Utilities|Time|GetWorldDeltaSeconds) (Variables|Default|GetTurnSpeedAcc)))
      (Transformation|SetActorRotation (Variables|Default|GetOwnerCharacter) (Class|KismetMathLibrary|RInterptoConstant (Transformation|GetActorRotation (Variables|Default|GetOwnerCharacter)) target (Utilities|Time|GetWorldDeltaSeconds) (Variables|Default|GetTurnSpeed))))))