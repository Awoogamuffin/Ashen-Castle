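; Actor component that turns its owning character to face the mouse cursor.
; Every tick it deprojects the mouse position for player controller 0 and intersects that ray with the world Z = 0 plane mathematically, without a trace.
; LookAtTarget then rotates the character toward that point with pitch zeroed, so it stays upright.
; The plane is fixed at world zero, independent of the character's height or the ground.
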(event EventBeginPlay
  (|CallParentFunction))

(event EventTick
  (params (DeltaSeconds :type Float%20%28single-precision%29))
  (bind _returnvalue (Game|GetPlayerController 0))
  (bind (_worldlocation _worlddirection) (Game|Player|ConvertMouseLocationToWorldSpace _returnvalue))
  (bind _output_get (Variables|Default|SetCursorDistance (Math|Float|SafeDivide (* (.Z (Math|Vector|BreakVector _worldlocation)) -1.0) (.Z (Math|Vector|BreakVector _worlddirection)))))
  (CallFunction|LookatTarget (+ _worldlocation (* _worlddirection _output_get))))

(fn LookatTarget
  (params (TargetPosition :type Vector :default "0, 0, 0"))
  (bind _ownercharacter (Variables|Default|GetOwnerCharacter))
  (bind _returnvalue (Transformation|GetActorLocation _ownercharacter))
  (bind _returnvalue_2 (Math|Rotator|FindLookatRotation _returnvalue TargetPosition))
  (bind (_roll _pitch _yaw) (Math|Rotator|BreakRotator _returnvalue_2))
  (Transformation|SetActorRotation (Variables|Default|GetOwnerCharacter) (Math|Rotator|MakeRotator _roll 0.0 _yaw)))