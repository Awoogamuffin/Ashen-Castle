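; AC_LookDirector is a character component that chooses which look behaviour drives the owner.
; On BeginPlay it caches the owner's AC_CursorLook and AC_FaceMovement components.
; HandleLook delegates to face-movement look while sprinting and to cursor look otherwise.
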(event EventBeginPlay
  (|CallParentFunction)
  (Variables|Default|SetCursorLookAC (Actor|GetComponentbyClass (Variables|Default|GetOwnerCharacter) "/Game/Ashen/Core/Characters/ActorComponents/Look/AC_CursorLook.AC_CursorLook_C"))
  (Variables|Default|SetFaceLookAC (Actor|GetComponentbyClass (Variables|Default|GetOwnerCharacter) "/Game/Ashen/Core/Characters/ActorComponents/Look/AC_FaceMovement.AC_FaceMovement_C")))

(fn HandleLook
  (if (Variables|Default|GetIsSprinting)
    (Default|HandleLook (Variables|Default|GetFaceLookAC))
    (else
      (Default|HandleLook (Variables|Default|GetCursorLookAC)))))