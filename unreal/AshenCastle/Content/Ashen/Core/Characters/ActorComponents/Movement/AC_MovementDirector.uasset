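; AC_MovementDirector is an actor component that acts as a pass-through to the owning character's AC_Movement component.
; On BeginPlay it runs the parent logic, then finds and caches AC_Movement on the owner character.
; GetMaxSpeed and ApplyMovementInput forward their arguments directly to that cached component, adding no movement logic of their own.
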(event EventBeginPlay
  (|CallParentFunction)
  (Variables|Default|SetMovementAC (Actor|GetComponentbyClass (Variables|Default|GetOwnerCharacter) "/Game/Ashen/Core/Characters/ActorComponents/Movement/AC_Movement.AC_Movement_C")))

(fn GetMaxSpeed()
  (params (Base :type Float%20%28double-precision%29))
  (bind _maxspeed (Default|GetMaxSpeed (Variables|Default|GetMovementAC) Base))
  (return _maxspeed))

(fn ApplyMovementInput
  (params (Input :type ST%20Apply%20Movement%20Params%20Structure))
  (Default|ApplyMovementInput (Variables|Default|GetMovementAC) Input))