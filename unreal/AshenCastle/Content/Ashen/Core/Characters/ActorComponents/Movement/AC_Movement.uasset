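; AC_Movement is an actor component that turns directional input into movement on its owning character.
; ApplyMovementInput flattens the control rotation to yaw only, then feeds Direction X along its right vector and Y along its forward vector as forced movement input.
; BeginPlay only calls the parent, and GetMaxSpeed is an empty stub.
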(event EventBeginPlay
  (|CallParentFunction))

(fn ApplyMovementInput
  (params (Input :type ST%20Apply%20Movement%20Params%20Structure))
  (bind _direction (Utilities|Struct|BreakST_ApplyMovementParams Input))
  (bind _ownercharacter (Variables|Default|GetOwnerCharacter))
  (bind _ownercharacter_2 (Variables|Default|GetOwnerCharacter))
  (bind (_x _y) (Math|Vector2D|BreakVector2D _direction))
  (bind _returnvalue (Pawn|GetControlRotation _ownercharacter :!class /Script/Engine.Pawn))
  (bind _yaw (Math|Rotator|BreakRotator _returnvalue))
  (bind _returnvalue_2 (Math|Rotator|MakeRotator 0.0 0.0 _yaw))
  (Pawn|Input|AddMovementInput _ownercharacter_2 (Math|Vector|GetRightVector _returnvalue_2) _x true)
  (Pawn|Input|AddMovementInput _ownercharacter_2 (Math|Vector|GetForwardVector _returnvalue_2) _y true))

(fn GetMaxSpeed)